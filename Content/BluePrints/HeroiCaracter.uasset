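; HeroiCaracter is the 2D flipbook player hero, with horizontal movement, jump, kick and projectile attack.
; Tick picks jump, walk, idle, kick or attack flipbooks from movement and input flags, flipping the sprite by X velocity.
; Tagged pickup overlaps set power flags; Power01 unlocks the attack, which spawns ProjetilBluePrint at Arrow1.
; Hitting a tagged enemy while not kicking sets IsDead, which only prints a message.
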(event OnComponentBeginOverlap(CapsuleComponent)
  (params (OverlappedComponent :type Primitive%20Component%20Object%20Reference) (OtherActor :type Actor%20Object%20Reference) (OtherComp :type Primitive%20Component%20Object%20Reference) (OtherBodyIndex :type Integer) (bFromSweep :type Boolean) (SweepResult :type Hit%20Result%20Structure%20%28by%20ref%29))
  (if (Components|ComponentHasTag OtherComp "power_01")
    (Development|PrintString "power")
    (Variables|Default|Setpower_01 true)
    (else
      (Development|PrintString "power 2")
      (if (Components|ComponentHasTag OtherComp "power_02")
        (Variables|Default|Setpower_02 true)))))

(event EventBeginPlay)

(event EventTick
  (params (DeltaSeconds :type Float%20%28single-precision%29))
  (if (Variables|Default|GetisDead)
    (Development|PrintString "Morto"))
  (if (AI|Components|NavMovement|IsFalling (Variables|Character|GetCharacterMovement))
    (Sprite|SetFlipbook (Variables|Default|GetHeroiFlipbook) "/Game/Assets/Paper2D/Sprites/FlipBook/JumpFlipBook.JumpFlipBook")
    (Math|Float|CompareFloat (.X (Math|Vector|BreakVector (Transformation|GetVelocity))) 0.0 :!label _label
      (:>
        (Transformation|SetRelativeRotation (Variables|Default|GetHeroiFlipbook) "0, 0, 0" false false))
      (:<
        (Transformation|SetRelativeRotation (Variables|Default|GetHeroiFlipbook) "0,180.000000, 0" false false)))
    (elif (> (Math|Vector|VectorLength (Transformation|GetVelocity)) 0.0)
      (Sprite|SetFlipbook (Variables|Default|GetHeroiFlipbook) "/Game/Assets/Paper2D/Sprites/FlipBook/AndarFlipBook.AndarFlipBook")
      (goto _label)
      (else
        (Sprite|SetFlipbook (Variables|Default|GetHeroiFlipbook) "/Game/Assets/Paper2D/Sprites/FlipBook/HeroiFlipbook.HeroiFlipbook")
        (if (Variables|Default|Getis_chute)
          (Sprite|SetFlipbook (Variables|Default|GetHeroiFlipbook) "/Game/Assets/Paper2D/Sprites/FlipBook/ChuteFlipBook.ChuteFlipBook")
          (Collision|SetCollisionObjectType (Variables|Default|GetHeroiFlipbook) "ECC_Pawn")
          (else
            (Sprite|SetFlipbook (Variables|Default|GetHeroiFlipbook) "/Game/Assets/Paper2D/Sprites/FlipBook/HeroiFlipbook.HeroiFlipbook")
            (if (Variables|Default|Getis_ataque)
              (Sprite|SetFlipbook (Variables|Default|GetHeroiFlipbook) "/Game/Assets/Paper2D/Sprites/FlipBook/AtaqueFlipBook.AtaqueFlipBook")
              (else
                (Sprite|SetFlipbook (Variables|Default|GetHeroiFlipbook) "/Game/Assets/Paper2D/Sprites/FlipBook/HeroiFlipbook.HeroiFlipbook")))))))))

(event Collision|EventHit
  (params (MyComp :type Primitive%20Component%20Object%20Reference) (Other :type Actor%20Object%20Reference) (OtherComp :type Primitive%20Component%20Object%20Reference) (bSelfMoved :type Boolean) (HitLocation :type Vector :default "0, 0, 0") (HitNormal :type Vector :default "0, 0, 0") (NormalImpulse :type Vector :default "0, 0, 0") (Hit :type Hit%20Result%20Structure%20%28by%20ref%29))
  (if (not (Variables|Default|Getis_chute))
    (if (Components|ComponentHasTag OtherComp "inimigo_01")
      (Variables|Default|SetisDead true))))

(event Input|ActionEvents|InputActionPular
  (params (Key :type Key%20Structure))
  (:Pressed
    (Character|Jump))
  (:Released
    (Character|StopJumping)))

(event Input|ActionEvents|InputActionChute
  (params (Key :type Key%20Structure))
  (:Pressed
    (Variables|Default|Setis_chute true))
  (:Released
    (Variables|Default|Setis_chute false)))

(event Input|ActionEvents|InputActionAtaque
  (params (Key :type Key%20Structure))
  (:Pressed
    (if (Variables|Default|Getpower_01)
      (Variables|Default|Setis_ataque true)))
  (:Released
    (Variables|Default|Setis_ataque false)))

(event Input|ActionEvents|InputActionAtaque
  (params (Key :type Key%20Structure))
  (:Pressed
    (if (Variables|Default|Getpower_01)
      (Game|SpawnActorfromClass "/Game/BluePrints/ProjetilBluePrint.ProjetilBluePrint_C" (Transformation|GetWorldTransform (Variables|Default|GetArrow1)) "Undefined" 0 0))))

(event Input|AxisEvents|InputAxismover
  (params (AxisValue :type Float%20%28single-precision%29))
  (Pawn|Input|AddMovementInput "1.000000, 0, 0" AxisValue false))

(fn ConstructionScript)