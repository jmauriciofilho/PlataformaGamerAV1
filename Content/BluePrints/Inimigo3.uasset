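; Inimigo3 is an enemy pawn that moves back and forth along the world X axis and can be killed.
; Each tick it applies movement input scaled by Movimento, and while nearly stopped a FlipFlop negates that value on every other firing.
; Capsule overlaps with components tagged "dano" print a debug message and subtract one Vida; Tick destroys the actor once Vida reaches zero.
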(event OnComponentBeginOverlap(CapsuleComponent)
  (params (OverlappedComponent :type Primitive%20Component%20Object%20Reference) (OtherActor :type Actor%20Object%20Reference) (OtherComp :type Primitive%20Component%20Object%20Reference) (OtherBodyIndex :type Integer) (bFromSweep :type Boolean) (SweepResult :type Hit%20Result%20Structure%20%28by%20ref%29))
  (if (Components|ComponentHasTag OtherComp "dano")
    (Development|PrintString "Dano")
    (Variables|Default|Setvida (- (Variables|Default|Getvida) 1))))

(event EventBeginPlay)

(event EventTick
  (params (DeltaSeconds :type Float%20%28single-precision%29))
  (if (<= (Variables|Default|Getvida) 0)
    (Actor|DestroyActor)
    (else
      (Utilities|FlowControl|Sequence
        (:then_0
          (Pawn|Input|AddMovementInput (Math|Vector|MakeVector 1.0 0.0 0.0) (Variables|Default|GetMovimento) false)
          (if (< (Math|Vector|VectorLength (Transformation|GetVelocity)) 1.0)
            (Utilities|FlowControl|FlipFlop
              (:A
                (Variables|Default|SetMovimento (* (Variables|Default|GetMovimento) -1.0)))
              (:B
                (Variables|Default|SetMovimento (* (Variables|Default|GetMovimento) 1.0))))))))))

(fn ConstructionScript)