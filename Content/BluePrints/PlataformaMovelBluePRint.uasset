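; Moving platform Blueprint that travels back and forth along the X axis while powered.
; Tick applies a frame-rate-independent offset, with the IsChoque flag setting the direction.
; Any actor begin-overlap toggles that flag to reverse the platform.
; When HeroiCaracter enters Box2, IsPower copies the hero's Power02 flag, so movement depends on that power.
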(event OnComponentBeginOverlap(Box2)
  (params (OverlappedComponent :type Primitive%20Component%20Object%20Reference) (OtherActor :type Actor%20Object%20Reference) (OtherComp :type Primitive%20Component%20Object%20Reference) (OtherBodyIndex :type Integer) (bFromSweep :type Boolean) (SweepResult :type Hit%20Result%20Structure%20%28by%20ref%29))
  (bind _asheroi_caracter (Utilities|Casting|CastToHeroiCaracter OtherActor))
  (Variables|Default|Setis_power (Variables|/Game/BluePrints/HeroiCaracter.HeroiCaracter_C|Getpower_02 _asheroi_caracter)))

(event EventBeginPlay)

(event EventTick
  (params (DeltaSeconds :type Float%20%28single-precision%29))
  (if (Variables|Default|Getis_power)
    (Transformation|AddActorWorldOffset (Math|Vector|MakeVector (* DeltaSeconds (Variables|Default|Getmovimento)) 0.0 0.0))
    (if (Variables|Default|Getis_choque)
      (Variables|Default|Setmovimento -1e+02)
      (else
        (Variables|Default|Setmovimento 1e+02)))))

(event Collision|EventActorBeginOverlap
  (params (OtherActor :type Actor%20Object%20Reference))
  (if (Variables|Default|Getis_choque)
    (Variables|Default|Setis_choque false)
    (else
      (Variables|Default|Setis_choque true))))

(fn ConstructionScript)